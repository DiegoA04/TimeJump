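; Checkpoint actor that records itself as the TimeTraveler player's latest checkpoint when the player overlaps its collider.
; It only replaces the stored checkpoint if none exists or if its CheckpointWeight is equal or higher, preventing regression to earlier checkpoints.
; On activation it swaps the static mesh material to green, and GetLocation exposes the sprite's world position.
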(event OnComponentBeginOverlap(Collider)
  (params (OverlappedComponent :type Primitive%20Component%20Object%20Reference) (OtherActor :type Actor%20Object%20Reference) (OtherComp :type Primitive%20Component%20Object%20Reference) (OtherBodyIndex :type Integer) (bFromSweep :type Boolean) (SweepResult :type Hit%20Result%20Structure%20%28by%20ref%29))
  (bind _astime_traveler_bp (Utilities|Casting|CastToTimeTraveler_BP OtherActor))
  (CallFunction|UpdateCheckpoint _astime_traveler_bp))

(fn ConstructionScript)

(fn GetLocation
  (return (Transformation|GetWorldLocation (Variables|Default|GetSpriteComponent self))))

(fn UpdateCheckpoint
  (params (PlayerCharacter :type Time%20Traveler%20BP%20Object%20Reference))
  (bind _lastcheckpoint (Default|GetLastCheckpoint PlayerCharacter))
  (if (Utilities|IsValid _lastcheckpoint)
    (if (<= (Variables|Checkpoint_BP_C|GetCheckpointWeight _lastcheckpoint) (Variables|Default|GetCheckpointWeight))
      (Default|SetLastCheckpoint PlayerCharacter self :!label _label)
      (Rendering|Material|SetMaterial (Variables|Default|GetStaticMesh) 0 "/Engine/EngineDebugMaterials/VertexColorViewMode_GreenOnly.VertexColorViewMode_GreenOnly"))
    (else
      (goto _label))))