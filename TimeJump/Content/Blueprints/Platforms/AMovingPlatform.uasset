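; AMovingPlatform is a platform actor that, while activated, shuttles back and forth along the world X, Y or Z axis chosen by its direction enum.
; Tick passes the axis to MovePlatform, which tracks an offset and flips direction at Range and zero.
; Move applies Speed per frame without delta-time scaling or sweep.
; The construction script assigns the configured mesh, and SetIsActivated toggles movement.
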(event EventTick
  (params (DeltaSeconds :type Float%20%28single-precision%29))
  ;[1 1 1] Continue if activated
  (if (Variables|Default|GetbIsActivated)
    ;[1 1 1] Determines Movement Direction
    (switch Utilities|FlowControl|Switch|SwitchonEDirection (Variables|Default|GetEDirection)
      (:NewEnumerator0
        (CallFunction|MovePlatform "1.000000, 0, 0"))
      (:NewEnumerator1
        (CallFunction|MovePlatform "0.000000,1.000000, 0"))
      (:NewEnumerator2
        (CallFunction|MovePlatform "0.000000, 0,1.000000")))))

(fn ConstructionScript
  (Components|StaticMesh|SetStaticMesh (Variables|Default|GetPlaceHolderMesh) (Variables|Default|GetPlatformMesh)))

(fn MovePlatform
  (params (DirectionVector :type Vector))
  (if (Variables|Default|GetbWasLastAtStart)
    (CallFunction|Move DirectionVector)
    (Variables|Default|SetCurrOffset (+ (Variables|Default|GetCurrOffset) (Variables|Default|GetSpeed)))
    (Variables|Default|SetbWasLastAtStart (< (Variables|Default|GetCurrOffset) (Variables|Default|GetRange)))
    (else
      (CallFunction|Move (* DirectionVector (Math|Float|SelectFloat -1.0 0.0 true)))
      (Variables|Default|SetCurrOffset (- (Variables|Default|GetCurrOffset) (Variables|Default|GetSpeed)))
      (Variables|Default|SetbWasLastAtStart (<= (Variables|Default|GetCurrOffset) 0)))))

(fn Move
  (params (DirectionVector :type Vector))
  (Transformation|SetActorLocation (+ (* DirectionVector (Variables|Default|GetSpeed)) (Transformation|GetActorLocation self)) false false))

(fn SetIsActivated
  (params (bShouldBeActivated :type Boolean))
  (CallFunction|SetIsActivated bShouldBeActivated))